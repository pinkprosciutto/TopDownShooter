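; Boss enemy that steers toward its target, attacks at close range, and reports its spawn and death to the top-down game mode.
; A looping timer drives flocking steering, pausing while a random attack runs: weapon burst, line-traced charge, explosion, or charge into explosion.
; Charges damage through repeated box traces, while explosions use scale timelines, a ground indicator and sphere traces.
; AI deactivation releases the weapon and interrupts charge and explosion.
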(event Custom|Timer_Steer
  (Class|ACFlockingAI|Steer (Variables|Default|GetAC_FlockingAI) (Transformation|GetActorLocation (CallFunction|GetTargetActor)) (Utilities|Array|MakeArray "ObjectTypeQuery1" "ObjectTypeQuery6") false 0.01)
  (CallFunction|CheckPlayerProximity))

(event Custom|OnDeactivateAI_Event
  (Utilities|Time|ClearTimerbyFunctionName 0 "Timer_Steer")
  (Utilities|Time|ClearTimerbyFunctionName 0 "Timer_ActivateWeapon")
  (CallFunction|ReleaseWeapon)
  (CallFunction|InterruptExplosion)
  (CallFunction|InterruptChargeAttack)
  (Variables|Data|SetIsAttackAvailable true)
  (Default|CallOnBossDeath (Variables|Default|GetAs%20BP%20Top%20Down%20Game%20Mode))
  (Variables|Data|SetIsDead true)
  (Variables|Default|SetIsActive false))

(event Custom|OnAttackFinished_Event
  (params (AttackCooldown :type Float%20%28double-precision%29))
  (Utilities|FlowControl|Delay AttackCooldown)
  (Variables|Data|SetIsAttackAvailable true))

(event Custom|IsAttacking_Event
  (Variables|Data|SetIsAttackAvailable false)
  (Class|KismetSystemLibrary|PauseTimer 0 "Timer_Steer"))

(event Custom|InitializeGameMode
  (bind _asbp_top_down_game_mode (Utilities|Casting|CastToBP_TopDownGameMode (Game|GetGameMode)))
  (Variables|Default|SetAs%20BP%20Top%20Down%20Game%20Mode _asbp_top_down_game_mode))

(event Custom|OnActivateAI_Event
  (Variables|Default|SetIsActive true)
  (Utilities|Time|SetTimerbyFunctionName 0 "Timer_Steer" 0.01 true)
  (Default|CallOnBossSpawn (Variables|Default|GetAs%20BP%20Top%20Down%20Game%20Mode))
  (Variables|Data|SetIsDead false))

(event Custom|CheckPlayerProximity
  ;[1 1 1] Check If Actor is close to Player
  (if (and (<= (Math|Vector|Distance(Vector) (Transformation|GetActorLocation (CallFunction|GetTargetActor)) (Transformation|GetActorLocation)) (Variables|Stats|GetTargetDistanceLimit)) (Variables|Data|GetIsAttackAvailable))
    (Class|KismetSystemLibrary|PauseTimer 0 "Timer_Steer")
    (CallFunction|QueueAttack)))

(event Custom|LookAtPlayer
  (bind _targetactor (CallFunction|GetTargetActor))
  (bind _returnvalue (Transformation|GetActorRotation))
  (bind _returnvalue_2 (Transformation|GetActorRotation))
  (bind _returnvalue_3 (Transformation|GetActorLocation _targetactor))
  (bind (_x _y) (Math|Vector|BreakVector _returnvalue_3))
  ;[1 1 1] Aim Towards Player
  (Transformation|SetActorRotation (Math|Rotator|MakeRotator (.roll _returnvalue) (.pitch _returnvalue) (.yaw (Math|Interpolation|RInterpTo (Transformation|GetActorRotation) (Math|Rotator|MakeRotator (.roll _returnvalue_2) (.pitch _returnvalue_2) (.yaw (Math|Rotator|FindLookatRotation (Transformation|GetActorLocation) (Math|Vector|MakeVector _x _y 1.5e+02)))) 0.01 (Variables|Stats|GetInterpSpeed))))))

(event EventBeginPlay
  (bind _explosiveradius (Variables|Stats|GetExplosiveRadius))
  (bind _returnvalue (/ _explosiveradius 55.0))
  (|CallParentFunction)
  (CallFunction|InitializeGameMode)
  (Utilities|FlowControl|Sequence
    (:then_0
      (Default|SpawnWeapon (Variables|Default|GetAC_WeaponAttachment) (Variables|Default|GetWeaponSocket))
      (EventDispatchers|AssignOnActivateAI (delegate Custom|OnActivateAI_Event))
      (EventDispatchers|AssignOnDeactivateAI (delegate Custom|OnDeactivateAI_Event))
      (Transformation|SetWorldScale3D (Variables|Default|GetAOE_Indicator) (Math|Vector|MakeVector _returnvalue _returnvalue 0.05)))
    (:then_1
      (bind _outactors (Actor|GetAllActorsOfClass "/Game/Blueprint/Characters/Enemy/BP_Enemy_Base.BP_Enemy_Base_C"))
      (bind _output_get (Variables|Data|SetIgnoredActors _outactors))
      (Default|SetIgnoredActors (Default|GetWeaponActor (Variables|Default|GetAC_WeaponAttachment)) _output_get))
    (:then_2
      (EventDispatchers|BindEventtoIsAttacking (delegate Custom|IsAttacking_Event))
      (EventDispatchers|BindEventtoOnAttackFinished (delegate Custom|OnAttackFinished_Event)))))

(event Custom|ChargeAttack
  (params (HasExplosion :type Boolean))
  ;[1 1 1] Charge Attack
  (Utilities|Time|SetTimerbyFunctionName 0 "LookAtPlayer" 0.01 true)
  (Utilities|FlowControl|Delay 1.5)
  (bind _outhit (Collision|LineTraceForObjects (Transformation|GetWorldLocation (Variables|Default|GetWeaponSocket)) (+ (Transformation|GetWorldLocation (Variables|Default|GetWeaponSocket)) (* (Transformation|GetActorForwardVector) 3e+03)) (Utilities|Array|MakeArray "ObjectTypeQuery1" "ObjectTypeQuery2") false 0 "None"))
  (Utilities|Time|ClearTimerbyFunctionName 0 "LookAtPlayer")
  (Utilities|Time|SetTimerbyFunctionName 0 "ComputeChargeHitbox" 0.05 true)
  (Components|MoveComponentTo (Variables|Default|GetDefaultSceneRoot) (Math|Vector|SelectVector (.ImpactPoint (Collision|BreakHitResult _outhit)) (.TraceEnd (Collision|BreakHitResult _outhit)) (.bBlockingHit (Collision|BreakHitResult _outhit))) (Transformation|GetActorRotation) false false 1.0 false)
  (Utilities|Time|ClearTimerbyFunctionName 0 "ComputeChargeHitbox")
  (if (not HasExplosion)
    (Utilities|FlowControl|Delay 1.0)
    (Class|KismetSystemLibrary|UnPauseTimer 0 "Timer_Steer")
    (Default|CallOnAttackFinished 1.0)
    (else
      (CallFunction|ExplosionAttack))))

(event Custom|ComputeChargeHitbox
  (bind _returnvalue (Transformation|GetActorLocation))
  ;[1 1 1] Charge Attack
  (bind _outhits (Class|KismetSystemLibrary|BoxTraceMultiforObjects _returnvalue _returnvalue "50.000000,50.000000,50.000000" "0, 0, 0" (Utilities|Array|MakeArray "ObjectTypeQuery7" "ObjectTypeQuery3") false 0 "None" true))
  (for _array_element _outhits
    (Default|CallOnDamage (Actor|GetComponentbyClass (.HitActor (Collision|BreakHitResult _array_element)) "/Script/TopDownShooter.AC_HealthSystem") (.ImpactPoint (Collision|BreakHitResult _array_element)) (Variables|Stats|GetChargeDamage) self)))

(event Custom|BasicShoot
  ;[1 1 1] Fire weapon at player
  (Utilities|Time|SetTimerbyFunctionName 0 "LookAtPlayer" 0.01 true)
  (Utilities|FlowControl|Delay 1.0)
  (CallFunction|FireWeapon)
  (Utilities|FlowControl|Delay 3.0)
  (CallFunction|ReleaseWeapon)
  (Class|KismetSystemLibrary|UnPauseTimer 0 "Timer_Steer")
  (Utilities|Time|ClearTimerbyFunctionName 0 "LookAtPlayer")
  (Default|CallOnAttackFinished 1.0))

(event Custom|QueueAttack
  (Default|CallIsAttacking)
  (switch int (Math|Random|RandomIntegerinRange 0 4)
    (:0
      (CallFunction|BasicShoot))
    (:1
      (CallFunction|ChargeAttack false))
    (:2
      (CallFunction|ExplosionAttack))
    (:3
      (CallFunction|ChargeAttack true))
    (:4
      (CallFunction|BasicShoot))))

(event Custom|InterruptExplosion
  ;[1 1 1] Explosion Attack
  (bind _sizechange (Timeline|PrimeExplosion Stop)
    (:Update
      (Transformation|SetWorldScale3D (Variables|Character|GetMesh) (* (Variables|Default|GetOriginalScale) _sizechange)))
    (:Finished
      (if (not (Variables|Data|GetIsDead))
        (CallFunction|Explode)
        (Development|SetHiddeninGame (Variables|Default|GetAOE_Indicator) true false)
        (bind _sizechange_2 (Timeline|ReturnScale PlayFromStart)
          (:Update
            (Transformation|SetWorldScale3D (Variables|Character|GetMesh) (* (Variables|Default|GetOriginalScale) _sizechange_2)))
          (:Finished
            (Utilities|FlowControl|Delay 1.0)
            (Class|KismetSystemLibrary|UnPauseTimer 0 "Timer_Steer")
            (Default|CallOnAttackFinished 1.0)))))))

(event Custom|InterruptChargeAttack
  ;[1 1 1] Charge Attack
  (Utilities|Time|ClearTimerbyFunctionName 0 "ComputeChargeHitbox")
  (Components|MoveComponentTo (Variables|Default|GetDefaultSceneRoot) (Math|Vector|SelectVector (.ImpactPoint (Collision|BreakHitResult (stale Custom|ChargeAttack _outhit))) (.TraceEnd (Collision|BreakHitResult (stale Custom|ChargeAttack _outhit))) (.bBlockingHit (Collision|BreakHitResult (stale Custom|ChargeAttack _outhit)))) (Transformation|GetActorRotation) false false 1.0 false) ; enters at Stop
)

(event Custom|ExplodeVFX
  ;[1 1 1] Explosion Attack
  (Niagara|SpawnSystematLocation "/Game/ArtAsset/Niagara/N_Explosion.N_Explosion" (Transformation|GetActorLocation)))

(event Custom|ShowExplosionIndicator
  (bind _returnvalue (Transformation|GetActorLocation))
  ;[1 1 1] Explosion Attack
  (bind _outhit (Collision|LineTraceForObjects _returnvalue (+ _returnvalue (* (Transformation|GetActorUpVector) -1.5e+04)) (Utilities|Array|MakeArray "ObjectTypeQuery1" "ObjectTypeQuery2") false 0 "None"))
  (Transformation|SetWorldLocation (Variables|Default|GetAOE_Indicator) (.ImpactPoint (Collision|BreakHitResult _outhit)) false false)
  (Development|SetHiddeninGame (Variables|Default|GetAOE_Indicator) false false))

(event Custom|FireWeapon
  ;[1 1 1] Fire weapon at player
  (if (not (Variables|Data|GetWeaponTriggerDown))
    (Class|IBPWeapon|OnFire (Default|GetWeaponActor (Variables|Default|GetAC_WeaponAttachment)))
    (Variables|Data|SetWeaponTriggerDown true)))

(event Custom|ReleaseWeapon
  ;[1 1 1] Fire weapon at player
  (if (Variables|Data|GetWeaponTriggerDown)
    (Class|IBPWeapon|OnRelease (Default|GetWeaponActor (Variables|Default|GetAC_WeaponAttachment)))
    (Variables|Data|SetWeaponTriggerDown false)))

(event Custom|Explode
  (bind _returnvalue (Transformation|GetActorLocation))
  (bind _returnvalue_2 (Transformation|GetActorLocation))
  ;[1 1 1] Explosion Attack
  (CallFunction|ExplodeVFX)
  (Utilities|FlowControl|Sequence
    (:then_0
      (bind _outhits (Collision|MultiSphereTraceForObjects _returnvalue_2 _returnvalue_2 (Variables|Stats|GetExplosiveRadius) (Utilities|Array|MakeArray "ObjectTypeQuery3") false (Utilities|Array|MakeArray self) "ForDuration" true "(R=1.000000,G=0.000000,B=0.000000,A=1.000000)" "(R=0.000000,G=1.000000,B=0.000000,A=1.000000)" 0.5))
      (for _array_element _outhits
        (Utilities|IsValid (Actor|GetComponentbyClass (.HitActor (Collision|BreakHitResult _array_element)) "/Script/TopDownShooter.AC_HealthSystem")
          (:Is%20Valid
            (Default|CallOnDamage (Actor|GetComponentbyClass (.HitActor (Collision|BreakHitResult _array_element)) "/Script/TopDownShooter.AC_HealthSystem") (.ImpactPoint (Collision|BreakHitResult _array_element)) (Variables|Stats|GetExplosiveDamage) self)))))
    (:then_1
      (bind _outhits_2 (Collision|MultiSphereTraceForObjects _returnvalue _returnvalue (Variables|Stats|GetExplosiveRadius) (Utilities|Array|MakeArray "ObjectTypeQuery7") false (Utilities|Array|MakeArray self) "ForDuration" true "(R=1.000000,G=0.000000,B=0.000000,A=1.000000)" "(R=0.000000,G=1.000000,B=0.000000,A=1.000000)" 0.5))
      (for _array_element_2 _outhits_2
        (Utilities|IsValid (Actor|GetComponentbyClass (.HitActor (Collision|BreakHitResult _array_element_2)) "/Script/TopDownShooter.AC_HealthSystem")
          (:Is%20Valid
            (Default|CallOnDamage (Actor|GetComponentbyClass (.HitActor (Collision|BreakHitResult _array_element_2)) "/Script/TopDownShooter.AC_HealthSystem") (.ImpactPoint (Collision|BreakHitResult _array_element_2)) 99999.0 self)))))))

(event Custom|ExplosionAttack
  ;[1 1 1] Explosion Attack
  (CallFunction|ShowExplosionIndicator)
  (bind _sizechange (Timeline|PrimeExplosion PlayFromStart)
    (:Update
      (Transformation|SetWorldScale3D (Variables|Character|GetMesh) (* (Variables|Default|GetOriginalScale) _sizechange)))
    (:Finished
      (if (not (Variables|Data|GetIsDead))
        (CallFunction|Explode)
        (Development|SetHiddeninGame (Variables|Default|GetAOE_Indicator) true false)
        (bind _sizechange_2 (Timeline|ReturnScale PlayFromStart)
          (:Update
            (Transformation|SetWorldScale3D (Variables|Character|GetMesh) (* (Variables|Default|GetOriginalScale) _sizechange_2)))
          (:Finished
            (Utilities|FlowControl|Delay 1.0)
            (Class|KismetSystemLibrary|UnPauseTimer 0 "Timer_Steer")
            (Default|CallOnAttackFinished 1.0)))))))

(fn ConstructionScript
  (|CallParentFunction))