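; Elite flocking drone enemy that steers toward its target around obstacles and fires an attached weapon when in range.
; On AI activation, fast looping timers drive the flocking component's steering and, after an initial delay, aim the weapon socket at the target at fixed height.
; A trigger flag prevents repeated fire and release calls.
; The weapon ignores enemies present at BeginPlay; deactivation stops timers, releases fire and decrements flock count.
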(event Custom|Timer_Steer
  (Class|ACFlockingAI|Steer (Variables|Default|GetAC_FlockingAI) (Transformation|GetActorLocation (CallFunction|GetTargetActor)) (Utilities|Array|MakeArray "ObjectTypeQuery1" "ObjectTypeQuery6") false 0.01))

(event Custom|OnDeactivateAI_Event
  (bind _ac_flockingai (Variables|Default|GetAC_FlockingAI))
  (Utilities|Time|ClearTimerbyFunctionName 0 "Timer_Steer")
  (Utilities|Time|ClearTimerbyFunctionName 0 "Timer_ActivateWeapon")
  (CallFunction|ReleaseWeapon)
  (Class|ACFlockingAI|SetFlockingCount _ac_flockingai (- (Class|ACFlockingAI|GetCurrentFlockingCount _ac_flockingai) 1)))

(event Custom|OnActivateAI_Event
  (Utilities|Time|SetTimerbyFunctionName 0 "Timer_Steer" 0.01 true)
  (Utilities|Time|SetTimerbyFunctionName 0 "Timer_ActivateWeapon" 0.01 true false (Variables|Default|GetInitialAttackDelay)))

(event Custom|Timer_ActivateWeapon
  (CallFunction|WeaponLookatPlayer))

(event Custom|Weapon_LookAtPlayer
  (bind _targetactor (CallFunction|GetTargetActor))
  (bind _returnvalue (Transformation|GetActorLocation _targetactor))
  (bind (_x _y) (Math|Vector|BreakVector _returnvalue))
  (Transformation|SetWorldRotation (Variables|Default|GetWeaponSocket) (Math|Rotator|FindLookatRotation (Transformation|GetWorldLocation (Variables|Default|GetWeaponSocket)) (Math|Vector|MakeVector _x _y 1.5e+02)) false false)
  (if (<= (Math|Vector|Distance(Vector) (Transformation|GetActorLocation (CallFunction|GetTargetActor)) (Transformation|GetActorLocation)) (Variables|Default|GetTargetDistanceLimit))
    (CallFunction|FireWeapon)
    (else
      (CallFunction|ReleaseWeapon))))

(event Custom|FireWeapon
  (if (not (Variables|Default|GetWeaponTriggerDown))
    (Class|IBPWeapon|OnFire (Default|GetWeaponActor (Variables|Default|GetAC_WeaponAttachment)))
    (Variables|Default|SetWeaponTriggerDown true)))

(event Custom|ReleaseWeapon
  (if (Variables|Default|GetWeaponTriggerDown)
    (Class|IBPWeapon|OnRelease (Default|GetWeaponActor (Variables|Default|GetAC_WeaponAttachment)))
    (Variables|Default|SetWeaponTriggerDown false)))

(event EventBeginPlay
  (|CallParentFunction)
  (Utilities|FlowControl|Sequence
    (:then_0
      (Default|SpawnWeapon (Variables|Default|GetAC_WeaponAttachment) (Variables|Default|GetWeaponSocket))
      (EventDispatchers|AssignOnActivateAI (delegate Custom|OnActivateAI_Event))
      (EventDispatchers|AssignOnDeactivateAI (delegate Custom|OnDeactivateAI_Event)))
    (:then_1
      (bind _outactors (Actor|GetAllActorsOfClass "/Game/Blueprint/Characters/Enemy/BP_Enemy_Base.BP_Enemy_Base_C"))
      (bind _output_get (Variables|Default|SetIgnoredActors _outactors))
      (Default|SetIgnoredActors (Default|GetWeaponActor (Variables|Default|GetAC_WeaponAttachment)) _output_get))))

(fn ConstructionScript
  (|CallParentFunction))