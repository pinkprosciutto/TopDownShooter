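; BP_Enemy_Base is the pooled enemy base that handles spawning, damage and death, targeting the player by default.
; Activation resets health, scales the mesh in through a timeline, then enables sphere collision and starts the AI.
; Damage feeds the health component, triggers a material flash and shows damage numbers through the owning BP_EnemyManager.
; Death stops collision and AI, plays a scale animation, then deactivates the enemy in its object pool for reuse.
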(event OnDamage(AC_HealthSystem)
  (params (hitLocation :type Vector :default "0, 0, 0") (damage :type Float%20%28single-precision%29) (damageCauser :type Actor%20Object%20Reference))
  (Class|ACHealthSystem|TakeDamage (Variables|Default|GetAC_HealthSystem) damage damageCauser)
  (Default|StartFlash (Variables|Default|GetAC_DamageFlash) 2.01 0.1)
  (Default|ShowDamageText (Variables|Data|GetSpawner) hitLocation (* (Math|Float|Truncate (* (* damage (Class|ACHealthSystem|GetDamageModifier (Variables|Default|GetAC_HealthSystem))) 1e+01)) 0.1)))

(event Death(AC_HealthSystem)
  (CallFunction|OnDeathEvent))

(event Custom|OnDeathEvent
  (Collision|SetCollisionEnabled (Variables|Default|GetSphere) "NoCollision")
  (Default|CallOnDeactivateAI)
  (bind _deathanim (Timeline|DeathAnim PlayFromStart)
    (:Update
      (Transformation|SetWorldScale3D (Variables|Default|GetMesh) (* (Variables|Data|GetOriginalScale) _deathanim)))
    (:Finished
      (Class|ACObjectPool|DeactivateObject (Variables|Default|GetObject%20Pool) (Variables|Data|GetObjectIndex))
      (Transformation|SetWorldScale3D (Variables|Default|GetMesh) (Variables|Data|GetOriginalScale)))))

(event EventInitializeObject
  (params (objectPool :type AC%20Object%20Pool%20Object%20Reference) (index :type Integer) (owner :type Actor%20Object%20Reference))
  (Variables|Default|SetObject%20Pool objectPool)
  (Variables|Data|SetObjectIndex index)
  (Default|InitiateDamageFlash (Variables|Default|GetAC_DamageFlash) (Variables|Default|GetMesh))
  (Variables|Data|SetOriginalScale (Transformation|GetWorldScale (Variables|Default|GetMesh)))
  (bind _asbp_enemy_manager (Utilities|Casting|CastToBP_EnemyManager owner))
  (Variables|Data|SetSpawner _asbp_enemy_manager))

(event EventOnActivate
  (params (position :type Vector :default "0, 0, 0") (rotation :type Rotator :default "0, 0, 0"))
  (Class|ACHealthSystem|InitializeHealth (Variables|Default|GetAC_HealthSystem) (Variables|Stats|GetMaxHealth))
  (bind _returnvalue (Actor|GetActorOfClass "/Game/Blueprint/Characters/BP_PlayerCharacter.BP_PlayerCharacter_C"))
  (Variables|Data|SetTargetActor _returnvalue)
  (Transformation|SetActorLocation position false false)
  (Rendering|SetActorHiddenInGame false)
  (bind _spawninscale (Timeline|SpawnAnim PlayFromStart)
    (:Update
      (Transformation|SetWorldScale3D (Variables|Default|GetMesh) (* (Variables|Data|GetOriginalScale) _spawninscale)))
    (:Finished
      (Collision|SetCollisionEnabled (Variables|Default|GetSphere) "QueryOnly")
      (Default|CallOnActivateAI))))

(event EventOnDeactivate
  (Actor|Tick|SetActorTickEnabled false)
  (Rendering|SetActorHiddenInGame true))

(fn ConstructionScript)

(fn GetTargetActor
  (return (Variables|Data|GetTargetActor)))

(fn SetNewTarget
  (params (NewActor :type BP%20Player%20Character%20Object%20Reference))
  (Variables|Data|SetTargetActor NewActor))