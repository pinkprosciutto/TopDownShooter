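; Kamikaze enemy that steers toward its target and self-destructs in a radial explosion when close or killed.
; On AI activation, looping timers drive flocking steering and proximity checks.
; Priming stops both timers, projects a radius-scaled warning indicator onto the ground and plays a mesh-scaling timeline.
; The blast spawns Niagara VFX, damages health components found by a sphere trace, then returns the enemy to its object pool.
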(event Custom|Timer_Steer
  ;[1 1 1] Initialization
  (Class|ACFlockingAI|Steer (Variables|Default|GetAC_FlockingAI) (Transformation|GetActorLocation (CallFunction|GetTargetActor)) (Utilities|Array|MakeArray "ObjectTypeQuery1" "ObjectTypeQuery6") false 0.01))

(event Custom|OnDeactivateAI_Event
  (bind _ac_flockingai (Variables|Default|GetAC_FlockingAI))
  ;[1 1 1] Initialization
  (Class|ACFlockingAI|SetFlockingCount _ac_flockingai (- (Class|ACFlockingAI|GetCurrentFlockingCount _ac_flockingai) 1)))

(event Custom|OnActivateAI_Event
  ;[1 1 1] Initialization
  (Utilities|Time|SetTimerbyFunctionName 0 "Timer_Steer" 0.01 true)
  (Utilities|Time|SetTimerbyFunctionName 0 "CheckPlayerProximity" 0.05 true))

(event Custom|ExplodeVFX
  (Niagara|SpawnSystematLocation "/Game/ArtAsset/Niagara/N_Explosion.N_Explosion" (Transformation|GetActorLocation)))

(event Custom|CheckPlayerProximity
  ;[1 1 1] Check If Actor is close to Player
  (if (<= (Math|Vector|Distance(Vector) (Transformation|GetActorLocation (CallFunction|GetTargetActor)) (Transformation|GetActorLocation)) 2e+02)
    (CallFunction|StartExplosionEvent)))

(event Custom|ShowExplosionIndicator
  (bind _returnvalue (Transformation|GetActorLocation))
  (bind _outhit (Collision|LineTraceForObjects _returnvalue (+ _returnvalue (* (Transformation|GetActorUpVector) -1.5e+04)) (Utilities|Array|MakeArray "ObjectTypeQuery1" "ObjectTypeQuery2") false 0 "None"))
  (Transformation|SetWorldLocation (Variables|Default|GetAOE_Indicator) (.ImpactPoint (Collision|BreakHitResult _outhit)) false false)
  (Development|SetHiddeninGame (Variables|Default|GetAOE_Indicator) false false))

(event Custom|Explode
  (bind _returnvalue (Transformation|GetActorLocation))
  ;[1 1 1] Prime Explosion Event
  (CallFunction|ExplodeVFX)
  (bind _outhits (Collision|MultiSphereTraceForObjects _returnvalue _returnvalue (Variables|Default|GetExplosiveRadius) (Utilities|Array|MakeArray "ObjectTypeQuery3" "ObjectTypeQuery7") false (Utilities|Array|MakeArray self) "ForDuration" true "(R=1.000000,G=0.000000,B=0.000000,A=1.000000)" "(R=0.000000,G=1.000000,B=0.000000,A=1.000000)" 0.5))
  (for _array_element _outhits
    (Utilities|IsValid (Actor|GetComponentbyClass (.HitActor (Collision|BreakHitResult _array_element)) "/Script/TopDownShooter.AC_HealthSystem")
      (:Is%20Valid
        (Default|CallOnDamage (Actor|GetComponentbyClass (.HitActor (Collision|BreakHitResult _array_element)) "/Script/TopDownShooter.AC_HealthSystem") (.ImpactPoint (Collision|BreakHitResult _array_element)) (Variables|Default|GetExplosiveDamage) self))))
  (Class|ACObjectPool|DeactivateObject (Variables|Default|GetObject%20Pool) (Variables|Default|GetObjectIndex)))

(event Custom|StartExplosionEvent
  ;[1 1 1] Prime Explosion Event
  (Utilities|Time|ClearTimerbyFunctionName 0 "CheckPlayerProximity")
  (Utilities|Time|ClearTimerbyFunctionName 0 "Timer_Steer")
  (Collision|SetCollisionEnabled (Variables|Default|GetSphere) "NoCollision")
  (CallFunction|ShowExplosionIndicator)
  (bind _sizechange (Timeline|StartExplosion PlayFromStart)
    (:Update
      (Transformation|SetWorldScale3D (Variables|Character|GetMesh) (* (Variables|Default|GetOriginalScale) _sizechange)))
    (:Finished
      (CallFunction|Explode)
      (Transformation|SetWorldScale3D (Variables|Character|GetMesh) (Variables|Default|GetOriginalScale))
      (Development|SetHiddeninGame (Variables|Default|GetAOE_Indicator) true false))))

(event EventBeginPlay
  (bind _explosiveradius (Variables|Default|GetExplosiveRadius))
  (bind _returnvalue (/ _explosiveradius 57.0))
  ;[1 1 1] Initialization
  (|CallParentFunction)
  (Utilities|FlowControl|Sequence
    (:then_0
      (EventDispatchers|AssignOnActivateAI (delegate Custom|OnActivateAI_Event))
      (Transformation|SetWorldScale3D (Variables|Default|GetAOE_Indicator) (Math|Vector|MakeVector _returnvalue _returnvalue 0.05))
      (EventDispatchers|AssignOnDeactivateAI (delegate Custom|OnDeactivateAI_Event)))))

(event EventOnDeathEvent
  ;[1 1 1] Prime Explosion Event
  (CallFunction|StartExplosionEvent)
  (Default|CallOnDeactivateAI))

(fn ConstructionScript
  (|CallParentFunction))