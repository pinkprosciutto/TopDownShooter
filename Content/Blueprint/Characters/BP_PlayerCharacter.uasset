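; Player pawn for a top-down shooter: moves by Enhanced Input, turns smoothly toward the mouse cursor and fires an attached weapon.
; A health component drives a camera-facing bar, scale animation, blinking invulnerability frames, paused regeneration and a death broadcast.
; Pickup collector events upgrade weapon stats, movement or regeneration, showing timed perk text.
; Boss spawn and death events add and remove a boss health bar.
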(event OnDamage(AC_HealthSystem)
  (params (hitLocation :type Vector :default "0, 0, 0") (damage :type Float%20%28single-precision%29) (damageCauser :type Actor%20Object%20Reference))
  (bind _ac_healthsystem (Variables|Default|GetAC_HealthSystem))
  (bind _currenthealth (Class|ACHealthSystem|GetCurrentHealth _ac_healthsystem))
  ;[1 1 1] On Damage Taken Event
  (if (Variables|Data|GetDamageable)
    (Class|ACHealthSystem|TakeDamage (Variables|Default|GetAC_HealthSystem) damage damageCauser)
    (Variables|Data|SetDamageable false)
    (Class|KismetSystemLibrary|PauseTimer 0 "RegenHealth")
    (Rendering|Material|SetScalarParameterValue (Variables|Data|GetDamageMaterial) "EmissiveMultiplier" 1.0 :!class /Script/Engine.MaterialInstanceDynamic)
    (Default|SetHealthPercent (Variables|Data|GetHealthWidget) _currenthealth)
    (if (> _currenthealth 0.0)
      (CallFunction|OnDamageAnim))))

(event Custom|LerpActorRotation
  (params (DeltaTime :type Float%20%28double-precision%29))
  (bind _returnvalue (Transformation|GetActorLocation))
  (bind _returnvalue_2 (Transformation|GetActorRotation))
  (bind _returnvalue_3 (Transformation|GetActorRotation))
  (bind _playercontroller (Variables|Data|GetPlayerController))
  (bind _hitresult (Game|Player|GetHitResultUnderCursorbyChannel _playercontroller "TraceTypeQuery1" true))
  (bind _location (Collision|BreakHitResult _hitresult))
  ;[1 1 1] Rotate Player
  (if (not (<= (Math|Vector|Distance(Vector) _location _returnvalue) (Variables|RotationData|GetCursorDistanceLimit)))
    (Transformation|SetActorRotation (Math|Rotator|MakeRotator (.roll _returnvalue_2) (.pitch _returnvalue_2) (.yaw (Math|Interpolation|RInterpTo (Transformation|GetActorRotation) (Math|Rotator|MakeRotator (.roll _returnvalue_3) (.pitch _returnvalue_3) (.yaw (Math|Rotator|FindLookatRotation (Math|Vector|MakeVector 0.0 0.0 0.0) (- _location _returnvalue)))) DeltaTime (Variables|RotationData|GetInterp%20Speed)))))))

(event Custom|StartIFrame
  ;[1 1 1] On Damage Taken Event
  (Utilities|FlowControl|FlipFlop
    (:A
      (Rendering|Material|SetScalarParameterValue (Variables|Data|GetDamageMaterial) "EmissiveMultiplier" 1.0 :!class /Script/Engine.MaterialInstanceDynamic))
    (:B
      (Rendering|Material|SetScalarParameterValue (Variables|Data|GetDamageMaterial) "EmissiveMultiplier" 0.0 :!class /Script/Engine.MaterialInstanceDynamic))))

(event Custom|StopIFrame
  ;[1 1 1] On Damage Taken Event
  (Rendering|Material|SetScalarParameterValue (Variables|Data|GetDamageMaterial) "EmissiveMultiplier" 0.0 :!class /Script/Engine.MaterialInstanceDynamic)
  (Utilities|Time|ClearTimerbyFunctionName 0 "StartIFrame")
  (Variables|Data|SetDamageable true)
  (Utilities|FlowControl|RetriggerableDelay 3.0)
  (Class|KismetSystemLibrary|UnPauseTimer 0 "RegenHealth"))

(event Custom|OnDamageAnim
  ;[1 1 1] On Damage Taken Event
  (bind _newtrack_0 (Timeline|DamageAnim PlayFromStart)
    (:Update
      (Transformation|SetWorldScale3D (Variables|Default|GetSphere) (* (Variables|Data|GetOriginalScale) _newtrack_0)))
    (:Finished
      (Utilities|Time|SetTimerbyFunctionName 0 "StartIFrame" 0.1 true)
      (Utilities|Time|SetTimerbyFunctionName 0 "StopIFrame" 1.0))))

(event Custom|OnBossSpawn_Event
  (bind _returnvalue (UserInterface|CreateWidget "/Game/Blueprint/Widget/WBP_BossHealthbar.WBP_BossHealthbar_C" (Game|GetPlayerController 0)))
  (UserInterface|Viewport|AddtoViewport _returnvalue 0)
  (Variables|Data|SetBossHealthBar _returnvalue))

(event Custom|OnBossDeath_Event
  (Widget|RemovefromParent (Variables|Data|GetBossHealthBar)))

(event Input|EnhancedActionEvents|EnhancedInputActionEscape
  (params (ActionValue :type Boolean) (ElapsedSeconds :type Float%20%28double-precision%29) (TriggeredSeconds :type Float%20%28double-precision%29) (InputAction :type Input%20Action%20Object%20Reference :default "/Game/Blueprint/Input/Escape.Escape"))
  ;[1 1 1] Input Event
  (:Started
    (Game|QuitGame 0 "Quit" false)))

(event Input|EnhancedActionEvents|EnhancedInputActionMovement
  (params (ActionValue :type Vector%202D%20Structure) (ElapsedSeconds :type Float%20%28double-precision%29) (TriggeredSeconds :type Float%20%28double-precision%29) (InputAction :type Input%20Action%20Object%20Reference :default "/Game/Blueprint/Input/Movement.Movement"))
  (bind _returnvalue (Pawn|GetControlRotation :!class /Script/Engine.Pawn))
  ;[1 1 1] Input Event
  (if (not (Variables|Default|GetIsDead))
    (Pawn|Input|AddMovementInput (Math|Vector|GetRightVector (Math|Rotator|MakeRotator (.roll _returnvalue) 0.0 (.yaw _returnvalue))) (.x ActionValue) false)
    (Pawn|Input|AddMovementInput (Math|Vector|GetForwardVector (Math|Rotator|MakeRotator 0.0 0.0 (.yaw (Pawn|GetControlRotation :!class /Script/Engine.Pawn)))) (.y ActionValue) false)))

(event Input|EnhancedActionEvents|EnhancedInputActionShoot
  (params (ActionValue :type Boolean) (ElapsedSeconds :type Float%20%28double-precision%29) (TriggeredSeconds :type Float%20%28double-precision%29) (InputAction :type Input%20Action%20Object%20Reference :default "/Game/Blueprint/Input/Shoot.Shoot"))
  ;[1 1 1] Input Event
  (:Started
    (if (not (Variables|Default|GetIsDead))
      (Class|IBPWeapon|OnFire (Default|GetWeaponActor (Variables|Default|GetAC_WeaponAttachment)))))
  (:Completed
    (Class|IBPWeapon|OnRelease (Default|GetWeaponActor (Variables|Default|GetAC_WeaponAttachment)))))

(event EventBeginPlay
  (CallFunction|InitializeHealth)
  (CallFunction|InitializePickupBehavior)
  (Variables|Data|SetOriginalScale (Transformation|GetWorldScale (Variables|Default|GetSphere)))
  (EventDispatchers|BindEventtoOnBossSpawn (delegate Custom|OnBossSpawn_Event))
  (EventDispatchers|BindEventtoOnBossDeath (delegate Custom|OnBossDeath_Event)))

(event EventTick
  (params (DeltaSeconds :type Float%20%28single-precision%29))
  ;[1 1 1] Rotate Player
  (CallFunction|LerpActorRotation DeltaSeconds))

(event Death(AC_HealthSystem)
  ;[1 1 1] On Death Event
  (CallFunction|OnDeath))

(event Custom|OnPossess
  ;[1 1 1] Possession
  (Utilities|FlowControl|Sequence
    (:then_0
      (bind _asplayer_controller (Utilities|Casting|CastToPlayerController (Pawn|GetController)))
      (Variables|Data|SetPlayerController _asplayer_controller)
      (Utilities|IsValid (PlayerController|LocalPlayerSubsystems|GetEnhancedInputLocalPlayerSubsystem _asplayer_controller)
        (:Is%20Valid
          (Input|AddMappingContext (PlayerController|LocalPlayerSubsystems|GetEnhancedInputLocalPlayerSubsystem _asplayer_controller) "/Game/Blueprint/Input/Input_PlayerMapping.Input_PlayerMapping" 0 "(bIgnoreAllPressedKeysUntilRelease=True,bForceImmediately=False,bNotifyUserSettings=False)")
          (Variables|/Script/Engine.PlayerController|SetbShowMouseCursor _asplayer_controller true))))
    (:then_1
      (Default|SpawnWeapon (Variables|Default|GetAC_WeaponAttachment) (Variables|Default|GetArrow)))))

(event Custom|AlignHealthBar
  ;[1 1 1] Initialize Health System
  (Transformation|SetWorldRotation (Variables|Default|GetHealthBar) (Math|Rotator|FindLookatRotation (Transformation|GetWorldLocation (Variables|Default|GetHealthBar)) (Transformation|GetActorLocation (Game|GetPlayerCameraManager 0))) false false))

(event Custom|RegenHealth
  (bind _ac_healthsystem (Variables|Default|GetAC_HealthSystem))
  (bind (_currenthealth _maxhealth) (Class|ACHealthSystem|GetCurrentHealth _ac_healthsystem))
  ;[1 1 1] Initialize Health System
  (Class|ACHealthSystem|SetCurrentHealth _ac_healthsystem (Math|Float|Clamp(Float) (+ (Variables|Stats|GetRegenSpeed) _currenthealth) 0.0 _maxhealth))
  (Default|SetHealthPercent (Variables|Data|GetHealthWidget) (.currentHealth (Class|ACHealthSystem|GetCurrentHealth (Variables|Default|GetAC_HealthSystem)))))

(event Custom|InitializeHealth
  (bind _floatingpawnmovement (Variables|Default|GetFloatingPawnMovement))
  (bind _sphere (Variables|Default|GetSphere))
  ;[1 1 1] Initialize Health System
  (Utilities|FlowControl|Sequence
    (:then_0
      (Class|ACHealthSystem|InitializeHealth (Variables|Default|GetAC_HealthSystem) (Variables|Stats|GetMaxHealth))
      (Variables|/Script/Engine.FloatingPawnMovement|SetMaxSpeed _floatingpawnmovement (Variables|Stats|GetMoveSpeed))
      (Variables|/Script/Engine.FloatingPawnMovement|SetAcceleration _floatingpawnmovement (Variables|Stats|GetMoveAcceleration))
      (bind _returnvalue (Rendering|Material|CreateDynamicMaterialInstance _sphere 0 (Rendering|Material|GetMaterial _sphere 0) "None" :!class /Script/Engine.PrimitiveComponent))
      (Variables|Data|SetDamageMaterial _returnvalue)
      (Utilities|Time|SetTimerbyFunctionName 0 "AlignHealthBar" 0.01 true))
    (:then_1
      (bind _aswbp_health_bar (Utilities|Casting|CastToWBP_HealthBar (UserInterface|GetWidget (Variables|Default|GetHealthBar))))
      (bind _output_get (Variables|Data|SetHealthWidget _aswbp_health_bar))
      (Rendering|SetCastShadow (Variables|Default|GetHealthBar) false)
      (Default|SetHealthPercent _output_get (Variables|Stats|GetMaxHealth)))))

(event Custom|InitializePickupBehavior
  ;[1 1 1] Initialize Perk System
  (EventDispatchers|AssignOnStatsUpdated (Variables|Default|GetAC_PickupCollector) (delegate Custom|OnStatsUpdated_Event))
  (bind _aswbp_perk_text (Utilities|Casting|CastToWBP_PerkText (UserInterface|GetWidget (Variables|Default|GetPerkText))))
  (Variables|Data|SetAs%20WBP%20Perk%20Text _aswbp_perk_text)
  (Rendering|SetCastShadow (Variables|Default|GetPerkText) false))

(event Custom|OnStatsUpdated_Event
  (params (PickupType :type E_Pickups%20Enum :default "NewEnumerator0") (PickupTier :type Integer) (Value :type Float%20%28double-precision%29) (IsTierMaxed :type Boolean))
  (bind _ac_weaponattachment (Variables|Default|GetAC_WeaponAttachment))
  (bind _floatingpawnmovement (Variables|Default|GetFloatingPawnMovement))
  (bind _weapon (Default|GetWeaponActor _ac_weaponattachment))
  ;[1 1 1] Initialize Perk System
  (Variables|Data|SetIs%20Tier%20Maxed IsTierMaxed)
  (Variables|Data|SetPickup%20Tier PickupTier)
  (Variables|Data|SetPickup%20Value Value)
  (switch Utilities|FlowControl|Switch|SwitchonE_Pickups PickupType
    (:NewEnumerator0
      (Default|IncreaseProjectileCount (Default|GetWeaponActor (Variables|Default|GetAC_WeaponAttachment)) (Variables|Data|GetPickup%20Value))
      (CallFunction|ObtainPerkText "Multishot" (Variables|Data|GetPickup%20Tier) (Variables|Data|GetIs%20Tier%20Maxed)))
    (:NewEnumerator1
      (Default|IncreaseFireRate _weapon (Variables|Data|GetPickup%20Value))
      (CallFunction|ObtainPerkText "Fire Rate" (Variables|Data|GetPickup%20Tier) (Variables|Data|GetIs%20Tier%20Maxed)))
    (:NewEnumerator2
      (Default|IncreaseDamage _weapon (Variables|Data|GetPickup%20Value))
      (CallFunction|ObtainPerkText "Damage" (Variables|Data|GetPickup%20Tier) (Variables|Data|GetIs%20Tier%20Maxed)))
    (:NewEnumerator3
      (Default|IncreaseProjectilePierceCount _weapon (Variables|Data|GetPickup%20Value))
      (CallFunction|ObtainPerkText "Bullet Pierce" (Variables|Data|GetPickup%20Tier) (Variables|Data|GetIs%20Tier%20Maxed)))
    (:NewEnumerator4
      (Variables|Stats|SetMoveSpeed (+ (Variables|Stats|GetMoveSpeed) (Math|Float|SelectFloat 0.0 (Variables|Data|GetPickup%20Value) (Variables|Data|GetIs%20Tier%20Maxed))))
      (Variables|Stats|SetMoveAcceleration (+ (Variables|Stats|GetMoveAcceleration) (Math|Float|SelectFloat 0.0 (Variables|Data|GetPickup%20Value) (Variables|Data|GetIs%20Tier%20Maxed))))
      (Variables|/Script/Engine.FloatingPawnMovement|SetMaxSpeed _floatingpawnmovement (Variables|Stats|GetMoveSpeed))
      (Variables|/Script/Engine.FloatingPawnMovement|SetAcceleration _floatingpawnmovement (Variables|Stats|GetMoveAcceleration))
      (CallFunction|ObtainPerkText "Move Speed" (Variables|Data|GetPickup%20Tier) (Variables|Data|GetIs%20Tier%20Maxed)))
    (:NewEnumerator5
      (Variables|Stats|SetRegenSpeed (+ (Variables|Stats|GetRegenSpeed) (Math|Float|SelectFloat 0.0 (Variables|Data|GetPickup%20Value) (Variables|Data|GetIs%20Tier%20Maxed))))
      (CallFunction|ObtainPerkText "Health Regen" (Variables|Data|GetPickup%20Tier) (Variables|Data|GetIs%20Tier%20Maxed))
      (Utilities|FlowControl|DoOnce false
        (:Completed
          (Utilities|Time|SetTimerbyFunctionName 0 "RegenHealth" 0.015 true))))))

(event Custom|ObtainPerkText
  (params (Text :type String) (Tier :type Integer) (IsTierMaxed :type Boolean))
  ;[1 1 1] Initialize Perk System
  (Transformation|SetWorldRotation (Variables|Default|GetPerkText) (Math|Rotator|FindLookatRotation (Transformation|GetWorldLocation (Variables|Default|GetPerkText)) (Transformation|GetActorLocation (Game|GetPlayerCameraManager 0))) false false)
  (Development|SetHiddeninGame (Variables|Default|GetPerkText) false false)
  (Default|PerkObtained (Variables|Data|GetAs%20WBP%20Perk%20Text) (Utilities|String|SelectText (Utilities|Text|ToText(String) (Utilities|String|Append Text " Maxed")) (Utilities|Text|ToText(String) (Utilities|String|Append Text " T" (Utilities|String|ToString(Integer) Tier))) IsTierMaxed))
  (Utilities|FlowControl|RetriggerableDelay 1.0)
  (Development|SetHiddeninGame (Variables|Default|GetPerkText) true false))

(event Custom|OnDeath
  ;[1 1 1] On Death Event
  (Actor|Tick|SetActorTickEnabled false)
  (Collision|SetCollisionEnabled (Variables|Default|GetHitbox) "NoCollision")
  (Utilities|Time|ClearTimerbyFunctionName 0 "RegenHealth")
  (Development|SetHiddeninGame (Variables|Default|GetHealthBar) true false)
  (Class|IBPWeapon|OnRelease (Default|GetWeaponActor (Variables|Default|GetAC_WeaponAttachment)))
  (bind _deathanim (Timeline|Timeline PlayFromStart)
    (:Update
      (Transformation|SetWorldScale3D (Variables|Default|GetSphere) (* (Variables|Data|GetOriginalScale) _deathanim)))
    (:Finished
      (Default|CallOnPlayerDeath)
      (Variables|Default|SetIsDead true))))

(fn ConstructionScript)