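; Enemy manager that runs escalating waves of flocker and kamikaze enemies, with elites, a boss, perk drops and damage text.
; Enemies, perks and text come from object pools, and spawned groups receive flocking and damage-modifier settings.
; Pool-return events count deaths and trigger the next wave, which grows flock sizes, then multi-waves and elite odds after the flocker cap.
; Perks drop by chance, from elites, or as a wave-end fallback.
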(event Custom|SpawnPerk
  (params (Location :type Vector) (Rotation :type Rotator))
  ;[1 1 1] Perk spawning
  (if (<= (Math|Random|RandomFloatinRange 0.0 1e+02) (Variables|EnemyData|GetPerkSpawnChance))
    (Class|ACObjectPool|ActivateObject (Variables|Default|GetAC_PerkPool) Location Rotation)
    (Variables|EnemyData|SetPerkSpawned? true)))

(event Custom|SpawnBoss
  ;[1 1 1] Enemy spwaning logic
  (bind _activatedactor (Class|ACObjectPool|ActivateObject (Variables|Default|GetAC_BossPool) (Variables|EnemyData|GetSelectedSpawnLoc) "0, 0, 0"))
  (Utilities|FlowControl|Sequence
    (:then_0
      (Class|ACFlockingAI|InitiateFlock (Actor|GetComponentbyClass _activatedactor "/Script/TopDownShooter.AC_FlockingAI") "0, 0, 0" (Variables|EnemyData|GetWaveID) 0 (Variables|EnemyData|GetSpawnedActors) 155.0))
    (:then_1
      (Utilities|IsValid (Actor|GetComponentbyClass _activatedactor "/Script/TopDownShooter.AC_HealthSystem")
        (:Is%20Valid
          (Class|ACHealthSystem|SetDamageModifier (Actor|GetComponentbyClass _activatedactor "/Script/TopDownShooter.AC_HealthSystem") (Variables|EnemyData|GetCurrentDmgModifier)))))))

(event Custom|SpawnKamikazeWave
  ;[1 1 1] Wave spawning logic
  (CallFunction|SpawnEnemy (Variables|Default|GetAC_KamikazePool) (Variables|KamikazeData|GetMinKamikazeCount) (Variables|KamikazeData|GetMaxKamikazeCount)))

(event Custom|SpawnNewWave
  (params (isBossWave :type Boolean))
  ;[1 1 1] Wave spawning logic
  (if (not isBossWave)
    (Variables|EnemyData|SetCurrentDmgModifier (Math|Float|Clamp(Float) (- (Variables|EnemyData|GetCurrentDmgModifier) (Math|Float|SelectFloat 0.04 0.01 (Variables|EnemyData|GetCapReached))) (Variables|EnemyData|GetMinimumDmgModifier)))
    (Utilities|FlowControl|Delay 1.0)
    (else
      (CallFunction|SpawnBoss)
      (Utilities|FlowControl|Delay 15.0)))
  (Variables|FlockData|SetFlockerSpawned false)
  (Variables|KamikazeData|SetKamikazeSpawned false)
  (for _index (range 0 (- (Variables|EnemyData|GetMultiWave) 1))
    (if (<= (Math|Random|RandomFloatinRange 0.0 1e+02) 7e+01)
      (CallFunction|SpawnFlockerWave)
      (Variables|FlockData|SetFlockerSpawned true)
      (else
        (CallFunction|SpawnKamikazeWave)
        (Variables|KamikazeData|SetKamikazeSpawned true))))
  (Utilities|FlowControl|Sequence
    (:then_0
      (if (Variables|EnemyData|GetCapReached)
        (Variables|EnemyData|SetMultiWave (Math|Integer|Clamp(Integer) (+ (Variables|EnemyData|GetMultiWave) 1) 0 (Variables|EnemyData|GetMaxMultiWave)))
        (Variables|Default|SetEliteSpawnChance (Math|Float|Clamp(Float) (+ (Variables|Default|GetEliteSpawnChance) 2.5) 0.0 1e+02))))
    (:then_1
      (if (Variables|FlockData|GetFlockerSpawned)
        (CallFunction|IncrementFlockerCount)))
    (:then_2
      (if (Variables|KamikazeData|GetKamikazeSpawned)
        (CallFunction|IncrementKamikazeCount)))))

(event Custom|IncrementFlockerCount
  ;[1 1 1] Increase Wave Density
  (Variables|FlockData|SetMinFlockCount (+ (Variables|FlockData|GetMinFlockCount) (Math|Integer|SelectInt 1 0 (< (Variables|FlockData|GetMinFlockCount) (- (Variables|FlockData|GetFlockerCountCap) 5)))))
  (Variables|FlockData|SetMaxFlockCount (+ (Variables|FlockData|GetMaxFlockCount) (Math|Integer|SelectInt 1 0 (< (Variables|FlockData|GetMaxFlockCount) (Variables|FlockData|GetFlockerCountCap)))))
  (Variables|EnemyData|SetCapReached (not (< (Variables|FlockData|GetMaxFlockCount) (Variables|FlockData|GetFlockerCountCap)))))

(event Custom|IncrementKamikazeCount
  ;[1 1 1] Increase Wave Density
  (Variables|KamikazeData|SetMinKamikazeCount (+ (Variables|KamikazeData|GetMinKamikazeCount) (Math|Integer|SelectInt 1 0 (< (Variables|KamikazeData|GetMinKamikazeCount) (- (Variables|KamikazeData|GetKamikazeCountCap) 1)))))
  (Variables|KamikazeData|SetMaxKamikazeCount (+ (Variables|KamikazeData|GetMaxKamikazeCount) (Math|Integer|SelectInt 1 0 (< (Variables|KamikazeData|GetMinKamikazeCount) (Variables|KamikazeData|GetKamikazeCountCap))))))

(event Custom|InitiateEnemy
  ;[1 1 1] Enemy spwaning logic
  (for _array_element (Variables|EnemyData|GetSpawnedActors)
    (Math|Integer|IncrementInt (Variables|EnemyData|GetCurrentEnemyCount)
      (:%20%20
        (Utilities|FlowControl|Sequence
          (:then_0
            (Utilities|IsValid (Actor|GetComponentbyClass _array_element "/Script/TopDownShooter.AC_FlockingAI")
              (:Is%20Valid
                (Class|ACFlockingAI|InitiateFlock (Actor|GetComponentbyClass _array_element "/Script/TopDownShooter.AC_FlockingAI") (Variables|EnemyData|GetSelectedSpawnLoc) (Variables|EnemyData|GetWaveID) (+ (Utilities|Array|LastIndex (Variables|EnemyData|GetSpawnedActors)) 1) (Variables|EnemyData|GetSpawnedActors) 155.0))))
          (:then_1
            (Utilities|IsValid (Actor|GetComponentbyClass _array_element "/Script/TopDownShooter.AC_HealthSystem")
              (:Is%20Valid
                (Class|ACHealthSystem|SetDamageModifier (Actor|GetComponentbyClass _array_element "/Script/TopDownShooter.AC_HealthSystem") (Variables|EnemyData|GetCurrentDmgModifier)))))))))
  (Utilities|Array|Clear (Variables|EnemyData|GetSpawnedActors))
  (Math|Integer|IncrementInt (Variables|EnemyData|GetWaveID)))

(event Custom|SpawnElite
  (params (ObjectPool :type AC%20Object%20Pool%20Object%20Reference))
  ;[1 1 1] Enemy spwaning logic
  (if (Variables|EnemyData|GetCapReached)
    (if (<= (Math|Random|RandomFloatinRange 0.0 1e+02) (Variables|Default|GetEliteSpawnChance))
      (if (== (Variables|Default|GetAC_FlockerPool) ObjectPool)
        (bind _activatedactor (Class|ACObjectPool|ActivateObject (Variables|Default|GetAC_EliteFlockerPool) (Variables|EnemyData|GetSelectedSpawnLoc) "0, 0, 0"))
        (Utilities|Array|Add (Variables|EnemyData|GetSpawnedActors) _activatedactor)
        (elif (== ObjectPool (Variables|Default|GetAC_KamikazePool))
          (bind _activatedactor_2 (Class|ACObjectPool|ActivateObject (Variables|Default|GetAC_EliteKamikazePool) (Variables|EnemyData|GetSelectedSpawnLoc) "0, 0, 0"))
          (Utilities|Array|Add (Variables|EnemyData|GetSpawnedActors) _activatedactor_2))))))

(event Custom|UpdateWaveStatus
  ;[1 1 1] Check current wave status
  (bind _result (Math|Integer|DecrementInt (Variables|EnemyData|GetCurrentEnemyCount))
    (:%20%20
      (if (<= _result 0)
        (Utilities|FlowControl|Sequence
          (:then_0
            (Default|CallSpawnNextWave))
          (:then_1
            (if (not (Variables|EnemyData|GetPerkSpawned?))
              (CallFunction|ForcedSpawnPerk)
              (else
                (Variables|EnemyData|SetPerkSpawned? false)))))))))

(event Custom|ForcedSpawnPerk
  ;[1 1 1] Perk spawning
  (Variables|EnemyData|SetPerkSpawned? false)
  (Class|ACObjectPool|ActivateObject (Variables|Default|GetAC_PerkPool) (Variables|EnemyData|GetLastKillLocation) (Variables|EnemyData|GetLastKillRotation)))

(event Custom|SpawnEnemy
  (params (SelectedPool :type AC%20Object%20Pool%20Object%20Reference) (MinFlockSize :type Integer) (MaxFlockSize :type Integer))
  ;[1 1 1] Enemy spwaning logic
  (Utilities|FlowControl|Sequence
    (:then_0
      (Variables|EnemyData|SetPerkSpawned? false)
      (Variables|EnemyData|SetSelectedSpawnLoc (Transformation|GetActorLocation (.OutItem (Utilities|Array|Random (Variables|EnemyData|GetSpawners)))))
      (for _index (range 0 (- (Math|Random|RandomIntegerinRange MinFlockSize MaxFlockSize) 1))
        (bind _activatedactor (Class|ACObjectPool|ActivateObject SelectedPool (Variables|EnemyData|GetSelectedSpawnLoc) "0, 0, 0"))
        (Utilities|Array|Add (Variables|EnemyData|GetSpawnedActors) _activatedactor))
      (CallFunction|SpawnElite SelectedPool)
      (CallFunction|InitiateEnemy))))

(event Custom|SpawnFlockerWave
  ;[1 1 1] Wave spawning logic
  (CallFunction|SpawnEnemy (Variables|Default|GetAC_FlockerPool) (Variables|FlockData|GetMinFlockCount) (Variables|FlockData|GetMaxFlockCount)))

(event EventBeginPlay
  (Utilities|FlowControl|Sequence
    (:then_0
      (CallFunction|InitializePerkPool))
    (:then_1
      (CallFunction|InitializeDamageTextPool)
      (CallFunction|InitializeEnemy)
      (Utilities|FlowControl|Delay 1.0)
      (CallFunction|SpawnEnemy (Variables|Default|GetAC_FlockerPool) (Variables|FlockData|GetMinFlockCount) (Variables|FlockData|GetMaxFlockCount)))))

(event Collision|EventActorBeginOverlap
  (params (OtherActor :type Actor%20Object%20Reference)))

(event EventTick
  (params (DeltaSeconds :type Float%20%28single-precision%29)))

(event Custom|BossDespawned
  (params (actor :type Actor%20Object%20Reference))
  ;[1 1 1] Start spawning enemies in pool
  (Default|CallBossDestroyed))

(event Custom|FlockerDespawned
  (params (actor :type Actor%20Object%20Reference))
  ;[1 1 1] Start spawning enemies in pool
  (CallFunction|OnEnemyDeath actor))

(event Custom|OnEnemyDeath
  (params (Actor :type Actor%20Object%20Reference))
  (bind _returnvalue (Transformation|GetActorLocation Actor))
  (Variables|EnemyData|SetLastKillLocation _returnvalue)
  (Variables|EnemyData|SetLastKillRotation (Transformation|GetActorRotation Actor))
  (CallFunction|SpawnPerk _returnvalue "0, 0, 0")
  (CallFunction|UpdateWaveStatus))

(event Custom|EliteKamikazeDespawned
  (params (actor :type Actor%20Object%20Reference))
  ;[1 1 1] Start spawning enemies in pool
  (CallFunction|OnEnemyDeath actor)
  (Class|ACObjectPool|ActivateObject (Variables|Default|GetAC_PerkPool) (Transformation|GetActorLocation actor) (Transformation|GetActorRotation actor)))

(event Custom|EliteFlockerDespawned
  (params (actor :type Actor%20Object%20Reference))
  ;[1 1 1] Start spawning enemies in pool
  (CallFunction|OnEnemyDeath actor)
  (Class|ACObjectPool|ActivateObject (Variables|Default|GetAC_PerkPool) (Transformation|GetActorLocation actor) (Transformation|GetActorRotation actor)))

(event Custom|InitializeEnemy
  ;[1 1 1] Start spawning enemies in pool
  (Utilities|FlowControl|Sequence
    (:then_0
      (Class|ACObjectPool|SpawnPool (Variables|Default|GetAC_FlockerPool) self)
      (Class|ACObjectPool|SpawnPool (Variables|Default|GetAC_KamikazePool) self)
      (Class|ACObjectPool|SpawnPool (Variables|Default|GetAC_EliteFlockerPool) self)
      (Class|ACObjectPool|SpawnPool (Variables|Default|GetAC_EliteKamikazePool) self)
      (bind _spawnedobjects (Class|ACObjectPool|SpawnPool (Variables|Default|GetAC_BossPool) self))
      (bind _asbp_enemy_boss (Utilities|Casting|CastToBP_Enemy_Boss (Utilities|Array|Get(acopy) _spawnedobjects)))
      (Variables|Default|SetBossAI _asbp_enemy_boss))
    (:then_1
      (bind _outactors (Actor|GetAllActorsOfClass "/Game/Blueprint/Manager/BP_EnemySpawner.BP_EnemySpawner_C"))
      (Variables|EnemyData|SetSpawners _outactors))
    (:then_2
      (EventDispatchers|BindEventtoPoolReturned (Variables|Default|GetAC_FlockerPool) (delegate Custom|FlockerDespawned))
      (EventDispatchers|BindEventtoPoolReturned (Variables|Default|GetAC_KamikazePool) (delegate Custom|KamikazeDespawned))
      (EventDispatchers|BindEventtoPoolReturned (Variables|Default|GetAC_EliteFlockerPool) (delegate Custom|EliteFlockerDespawned))
      (EventDispatchers|BindEventtoPoolReturned (Variables|Default|GetAC_EliteKamikazePool) (delegate Custom|EliteKamikazeDespawned))
      (EventDispatchers|BindEventtoPoolReturned (Variables|Default|GetAC_BossPool) (delegate Custom|BossDespawned)))
    (:then_3
      (EventDispatchers|BindEventtoSpawnNextWave (delegate Custom|SpawnNextWave_Event)))))

(event Custom|InitializePerkPool
  ;[1 1 1] Start spawning Perks
  (Class|ACObjectPool|SpawnPool (Variables|Default|GetAC_PerkPool) self))

(event Custom|InitializeDamageTextPool
  ;[1 1 1] Start spawning damage text
  (bind _spawnedobjects (Class|ACObjectPool|SpawnPool (Variables|Default|GetAC_DamageTextPool)))
  (for _array_element _spawnedobjects
    (bind _asbp_damage_text (Utilities|Casting|CastToBP_DamageText _array_element))
    (Utilities|Array|Add (Variables|DamageText|GetDamageTextPool) _asbp_damage_text)))

(event Custom|KamikazeDespawned
  (params (actor :type Actor%20Object%20Reference))
  ;[1 1 1] Start spawning enemies in pool
  (CallFunction|OnEnemyDeath actor))

(event Custom|SpawnNextWave_Event
  ;[1 1 1] Start spawning enemies in pool
  (if (and (>= (Variables|EnemyData|GetMultiWave) (Variables|EnemyData|GetMaxMultiWave)) (not (Variables|/Game/Blueprint/Characters/Enemy/BP_Enemy_Boss.BP_Enemy_Boss_C|GetIsActive (Variables|Default|GetBossAI))))
    (if (<= (Variables|Default|GetNewBossCountdown) 0)
      (CallFunction|SpawnNewWave true)
      (Variables|Default|SetNewBossCountdown 10)
      (else
        (CallFunction|SpawnNewWave false :!label _label)))
    (else
      (goto _label))))

(fn ConstructionScript)

(fn ShowDamageText
  (params (Location :type Vector) (Damage :type Float%20%28double-precision%29))
  (bind _activatedactor (Class|ACObjectPool|ActivateObject (Variables|Default|GetAC_DamageTextPool) Location "0, 0, 0"))
  (bind _asbp_damage_text (Utilities|Casting|CastToBP_DamageText _activatedactor))
  (Default|SetDamageText _asbp_damage_text Damage Location))