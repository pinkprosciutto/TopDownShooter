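; Base weapon that fires pooled BP_Projectiles from a socket, with upgradeable damage, fire rate, projectile count and pierce.
; InitializeProjectiles fills the pool from ACBulletPool and binds hit damage to each target's AC_HealthSystem.
; While fire is held, a looping timer counts down between volleys, activating projectiles with CalculateSpread rotations.
; InitializeData stores base stats, and upgrade functions set base plus value, pushing pierce changes to pooled projectiles.
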(event Custom|InitializeProjectiles
  (bind _spawnedobjects (Class|ACObjectPool|SpawnPool (Variables|Default|GetAC_BulletPool) (Components|GetOwner)))
  (for _array_element _spawnedobjects
    (bind _asbp_projectile (Utilities|Casting|CastToBP_Projectile _array_element))
    (Utilities|Array|Add (Variables|Data|GetProjectilePool) _asbp_projectile)
    (Default|InitializeStats _asbp_projectile (Variables|WeaponData|GetBaseProjectileRadius) (Variables|WeaponData|GetBaseProjectileSpeed) (Variables|WeaponData|GetBaseProjectileLifespan) (Variables|WeaponData|GetBaseProjectilePierceCount)))
  (EventDispatchers|BindEventtoOnDamage (delegate Custom|OnDamage_Event)))

(event Custom|WeaponFire
  (if (<= (Variables|Data|GetLastShotCountdown) 0.0)
    (for _index (range 0 (- (Variables|WeaponData|GetProjectileCount) 1))
      (Class|ACObjectPool|ActivateObject (Variables|Default|GetAC_BulletPool) (Transformation|GetWorldLocation (Variables|Default|GetSocket)) (Utilities|CalculateSpread _index))
      (Variables|Data|SetLastShotCountdown (/ 1.0 (Variables|WeaponData|GetFireRate))))
    (else
      (Variables|Data|SetLastShotCountdown (- (Variables|Data|GetLastShotCountdown) 0.01)))))

(event Custom|OnDamage_Event
  (params (HitResults :type Array%20of%20Hit%20Result%20Structures))
  (for _array_element HitResults
    (Utilities|IsValid (Actor|GetComponentbyClass (.HitActor (Collision|BreakHitResult _array_element)) "/Script/TopDownShooter.AC_HealthSystem")
      (:Is%20Valid
        (Default|CallOnDamage (Actor|GetComponentbyClass (.HitActor (Collision|BreakHitResult _array_element)) "/Script/TopDownShooter.AC_HealthSystem") (.ImpactPoint (Collision|BreakHitResult _array_element)) (Variables|WeaponData|GetProjectileDamage) (Components|GetOwner))))))

(event EventOnFire
  (Utilities|Time|SetTimerbyFunctionName 0 "WeaponFire" 0.01 true))

(event EventOnRelease
  (Utilities|Time|ClearTimerbyFunctionName 0 "WeaponFire"))

(fn ConstructionScript)

(fn InitializeData
  (params (ProjectileSpeed :type Float%20%28double-precision%29) (ProjectileLifespan :type Float%20%28double-precision%29) (ProjectileDamage :type Float%20%28double-precision%29) (ProjectileSpread :type Float%20%28double-precision%29) (ProjectileCount :type Integer) (ProjectileHitCount :type Integer) (ProjectileRadius :type Float%20%28double-precision%29) (MultishotAngleOffset :type Float%20%28double-precision%29) (FireRate :type Float%20%28double-precision%29))
  (Variables|WeaponData|SetBaseProjectileSpeed ProjectileSpeed)
  (Variables|WeaponData|SetBaseProjectileLifespan ProjectileLifespan)
  (bind _output_get (Variables|WeaponData|SetBaseProjectileDamage ProjectileDamage))
  (Variables|WeaponData|SetProjectileDamage _output_get)
  (Variables|WeaponData|SetBaseProjectileSpread ProjectileSpread)
  (bind _output_get_2 (Variables|WeaponData|SetBaseProjectileCountPerShot ProjectileCount))
  (Variables|WeaponData|SetProjectileCount _output_get_2)
  (bind _output_get_3 (Variables|WeaponData|SetBaseProjectilePierceCount ProjectileHitCount))
  (Variables|WeaponData|SetProjectilePierceCount _output_get_3)
  (Variables|WeaponData|SetBaseMultishotAngleOffset MultishotAngleOffset)
  (Variables|WeaponData|SetBaseProjectileRadius ProjectileRadius)
  (bind _output_get_4 (Variables|WeaponData|SetBaseFireRate FireRate))
  (Variables|WeaponData|SetFireRate _output_get_4))

(fn SetIgnoredActors
  (params (IgnoredActors :type Array%20of%20Actor%20Object%20References))
  (for _array_element (Variables|Data|GetProjectilePool)
    (Default|SetIgnoredActors _array_element IgnoredActors)))

(fn AppendIgnoredActors
  (params (AppendIgnoredActors :type Array%20of%20Actor%20Object%20References))
  (for _array_element (Variables|Data|GetProjectilePool)
    (Default|AppendIgnoredActors _array_element AppendIgnoredActors)))

(fn IncreaseProjectileCount
  (params (Value :type Float%20%28double-precision%29))
  (Variables|WeaponData|SetProjectileCount (Math|Float|Truncate (+ (Variables|WeaponData|GetBaseProjectileCountPerShot) Value)))
  (Development|PrintString "Projectile Count Increased" true true "(R=0.000000,G=0.660000,B=1.000000,A=1.000000)" 12.0))

(fn IncreaseProjectilePierceCount
  (params (Value :type Float%20%28double-precision%29))
  (bind _output_get (Variables|WeaponData|SetProjectilePierceCount (Math|Float|Truncate (+ (Variables|WeaponData|GetBaseProjectilePierceCount) Value))))
  (Development|PrintString "Pierce Count Increase")
  (for _array_element (Variables|Data|GetProjectilePool)
    (Variables|/Game/Blueprint/Weapons/Projectiles/BP_Projectile.BP_Projectile_C|SetProjectileHitCount _array_element _output_get)))

(fn IncreaseDamage
  (params (Value :type Float%20%28double-precision%29))
  (Variables|WeaponData|SetProjectileDamage (+ (Variables|WeaponData|GetBaseProjectileDamage) Value))
  (Development|PrintString "Projectile Damage Increase"))

(fn IncreaseFireRate
  (params (Value :type Float%20%28double-precision%29))
  (Variables|WeaponData|SetFireRate (+ (Variables|WeaponData|GetBaseFireRate) Value))
  (Development|PrintString "Projectile Fire Rate Increase"))