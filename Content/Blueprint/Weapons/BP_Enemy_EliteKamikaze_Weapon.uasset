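; Weapon Blueprint for the elite kamikaze enemy that fires a radial ring of bullets.
; On fire, it activates SpawnedBullets projectiles from its bullet pool component at the socket's world location.
; Each bullet's yaw steps by 360 divided by the count, in world space with zero pitch and roll, independent of the socket's rotation.
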(event EventOnFire
  (for _index (range 0 (- (Variables|Default|GetSpawnedBullets) 1))
    (Class|ACObjectPool|ActivateObject (Variables|Default|GetAC_BulletPool) (Transformation|GetWorldLocation (Variables|Default|GetSocket)) (Math|Rotator|MakeRotator 0.0 0.0 (Math|Conversions|ToFloat(Integer) (* _index (/ 360 (Variables|Default|GetSpawnedBullets))))))))

(fn ConstructionScript
  (|CallParentFunction))