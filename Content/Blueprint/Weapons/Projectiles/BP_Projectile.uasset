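; BP_Projectile is a pooled bullet actor that moves every tick and reports hits to the BP_Weapon_Base that owns it.
; On activation, looping timers run sphere-style collision checks at a fixed trace rate, ignoring the gun and its owner, and a lifespan timer returns it to the pool.
; Hits count toward a pierce limit, and pierce-blocker components end the bullet immediately.
; A front-of-muzzle check is present but unconnected.
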(event Custom|Timer_DeactivateBullet
  (Class|ACObjectPool|DeactivateObject (Variables|Default|GetObject%20Pool) (Variables|Data|GetActorIndex))
  (Utilities|Time|ClearTimerbyFunctionName 0 "Timer_DeactivateBullet")
  (Utilities|Time|ClearTimerbyFunctionName 0 "Timer_CheckCollision"))

(event Custom|Timer_CheckCollision
  (bind (_ishit _hitresult) (Class|Projectile|CheckCollision (Variables|Data|GetBulletRadius) false (Variables|Data|GetIgnoredActors) (Variables|Data|GetCollidableObject)))
  (if _ishit
    (Class|Projectile|OnBulletHit (Utilities|Array|MakeArray (Utilities|Array|Get(acopy) _hitresult)))))

(event Custom|InitializeStats
  (params (BulletRadius :type Float%20%28double-precision%29) (ProjectileSpeed :type Float%20%28double-precision%29) (ProjectileLifespan :type Float%20%28double-precision%29) (ProjectileHitCount :type Integer))
  (Variables|Data|SetBulletRadius BulletRadius)
  (Variables|Data|SetProjectileSpeed ProjectileSpeed)
  (Variables|Data|SetProjectileLifespan ProjectileLifespan)
  (Variables|Data|SetProjectileHitCount ProjectileHitCount))

(event EventOnBulletHit
  (params (hitResult :type Array%20of%20Hit%20Result%20Structures))
  (Default|CallOnDamage (Variables|Data|GetGunActor) hitResult)
  (Utilities|IsValid (Actor|GetComponentbyClass (.HitActor (Collision|BreakHitResult (Utilities|Array|Get(acopy) hitResult))) "/Game/Blueprint/Components/AC_PierceProjectileBlocker.AC_PierceProjectileBlocker_C")
    (:Is%20Valid
      (CallFunction|TimerDeactivateBullet :!label _label)
      (Variables|Default|SetCurrentHitCount 0))
    (:Is%20Not%20Valid
      (Math|Integer|IncrementInt (Variables|Default|GetCurrentHitCount)
        (:%20%20
          (if (>= (Variables|Default|GetCurrentHitCount) (Variables|Data|GetProjectileHitCount))
            (goto _label)))))))

(event EventOnActivate
  (params (position :type Vector :default "0, 0, 0") (rotation :type Rotator :default "0, 0, 0"))
  (Class|Projectile|ActivateBullet position rotation)
  (Utilities|Time|SetTimerbyFunctionName 0 "Timer_DeactivateBullet" (Variables|Data|GetProjectileLifespan))
  (Utilities|Time|SetTimerbyFunctionName 0 "Timer_CheckCollision" (/ 1.0 (Variables|Data|GetTracePerSecond)) true))

(event EventOnDeactivate
  (Class|Projectile|DeactivateBullet))

(event EventInitializeObject
  (params (objectPool :type AC%20Object%20Pool%20Object%20Reference) (index :type Integer) (owner :type Actor%20Object%20Reference))
  (Variables|Default|SetObject%20Pool objectPool)
  (Variables|Data|SetActorIndex index)
  (bind _asbp_weapon_base (Utilities|Casting|CastToBP_Weapon_Base owner))
  (Variables|Data|SetGunActor _asbp_weapon_base)
  (Utilities|Array|AppendArray (Variables|Data|GetIgnoredActors) (Utilities|Array|MakeArray (Variables|Data|GetGunActor) (Components|GetOwner (Variables|Data|GetGunActor)))))

(event EventTick
  (params (DeltaSeconds :type Float%20%28single-precision%29))
  (Class|Projectile|MoveBullet (Variables|Data|GetProjectileSpeed) DeltaSeconds))

(fn ConstructionScript)

(fn AppendIgnoredActors
  (params (NewActors :type Array%20of%20Actor%20Object%20References))
  (Utilities|Array|AppendArray (Variables|Data|GetIgnoredActors) NewActors))

(fn SetIgnoredActors
  (params (NewParam :type Array%20of%20Actor%20Object%20References))
  (Variables|Data|SetIgnoredActors NewParam))