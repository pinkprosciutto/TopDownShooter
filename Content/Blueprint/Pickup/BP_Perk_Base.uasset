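; Pooled perk pickup base that grants one of six randomly chosen perk types to actors with an AC_PickupCollector component.
; On activation it rolls a perk ID, tints the cube's dynamic material to match, enables box physics and applies a random bounce impulse.
; Overlapping a collector reports the perk and returns the actor to its pool.
; When its lifespan expires, collision switches off and a Timeline animates the cube's scale before pool deactivation.
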(event OnComponentBeginOverlap(Box)
  (params (OverlappedComponent :type Primitive%20Component%20Object%20Reference) (OtherActor :type Actor%20Object%20Reference) (OtherComp :type Primitive%20Component%20Object%20Reference) (OtherBodyIndex :type Integer) (bFromSweep :type Boolean) (SweepResult :type Hit%20Result%20Structure%20%28by%20ref%29))
  (bind _returnvalue (Actor|GetComponentbyClass OtherActor "/Game/Blueprint/Components/AC_PickupCollector.AC_PickupCollector_C"))
  (Utilities|IsValid _returnvalue
    (:Is%20Valid
      (Default|OnPickupCollected _returnvalue (Utilities|Enum|ByteToEnumE_Pickups (Math|Conversions|ToByte(Integer) (Variables|Default|GetPerkID))))
      (Class|ACObjectPool|DeactivateObject (Variables|Default|GetObject%20Pool) (Variables|Data|GetObjectIndex)))))

(event Custom|Bounce
  (Physics|AddImpulseatLocation (Variables|Default|GetBox) (* (Math|Random|RandomUnitVector) (Variables|Default|GetBounceStrength)) (+ (Transformation|GetActorLocation) (* (Transformation|GetActorUpVector) 5.05e+03)) "None"))

(event Custom|ActivateCollision
  (params (IsActive? :type Boolean))
  (bind _box (Variables|Default|GetBox))
  (Physics|SetSimulatePhysics _box IsActive?)
  (Collision|SetCollisionEnabled _box (select IsActive? "QueryAndPhysics" "NoCollision"))
  (Physics|SetEnableGravity _box IsActive?))

(event Custom|Timer_Despawn
  (Utilities|Time|ClearTimerbyFunctionName 0 "Timer_Despawn")
  (CallFunction|ActivateCollision false)
  (bind _scale (Timeline|Timeline PlayFromStart)
    (:Update
      (Transformation|SetWorldScale3D (Variables|Default|GetCube) (* (Variables|Default|GetOriginalScale) _scale)))
    (:Finished
      (Class|ACObjectPool|DeactivateObject (Variables|Default|GetObject%20Pool) (Variables|Data|GetObjectIndex)))))

(event Custom|RandomizePerkID
  (bind _output_get (Variables|Default|SetPerkID (Math|Random|RandomIntegerinRange 0 5)))
  (switch int _output_get
    (:0
      (Rendering|Material|SetVectorParameterValue (Variables|Default|GetMaterial) "EmissiveColor" "(R=0.744718,G=1.000000,B=0.067723,A=1.000000)" :!class /Script/Engine.MaterialInstanceDynamic))
    (:1
      (Rendering|Material|SetVectorParameterValue (Variables|Default|GetMaterial) "EmissiveColor" "(R=1.000000,G=0.000000,B=0.000000,A=1.000000)" :!class /Script/Engine.MaterialInstanceDynamic))
    (:2
      (Rendering|Material|SetVectorParameterValue (Variables|Default|GetMaterial) "EmissiveColor" "(R=1.000000,G=0.000000,B=0.750000,A=1.000000)" :!class /Script/Engine.MaterialInstanceDynamic))
    (:3
      (Rendering|Material|SetVectorParameterValue (Variables|Default|GetMaterial) "EmissiveColor" "(R=0.218554,G=0.000000,B=1.000000,A=1.000000)" :!class /Script/Engine.MaterialInstanceDynamic))
    (:4
      (Rendering|Material|SetVectorParameterValue (Variables|Default|GetMaterial) "EmissiveColor" "(R=0.000000,G=0.600626,B=1.000000,A=1.000000)" :!class /Script/Engine.MaterialInstanceDynamic))
    (:5
      (Rendering|Material|SetVectorParameterValue (Variables|Default|GetMaterial) "EmissiveColor" "(R=0.000000,G=1.000000,B=0.404889,A=1.000000)" :!class /Script/Engine.MaterialInstanceDynamic))))

(event EventOnActivate
  (params (position :type Vector :default "0, 0, 0") (rotation :type Rotator :default "0, 0, 0"))
  (Transformation|SetWorldScale3D (Variables|Default|GetCube) (Variables|Default|GetOriginalScale))
  (CallFunction|RandomizePerkID)
  (Transformation|SetActorLocation position false false)
  (Transformation|SetActorRotation rotation)
  (CallFunction|ActivateCollision true)
  (Rendering|SetActorHiddenInGame false)
  (CallFunction|Bounce)
  (Utilities|Time|SetTimerbyFunctionName 0 "Timer_Despawn" (Variables|Default|GetLifespan)))

(event EventOnDeactivate
  (CallFunction|ActivateCollision false)
  (Rendering|SetActorHiddenInGame true)
  (Utilities|Time|ClearTimerbyFunctionName 0 "Timer_Despawn"))

(event EventInitializeObject
  (params (objectPool :type AC%20Object%20Pool%20Object%20Reference) (index :type Integer) (owner :type Actor%20Object%20Reference))
  (Variables|Default|SetObject%20Pool objectPool)
  (Variables|Data|SetObjectIndex index)
  (CallFunction|ActivateCollision false))

(event EventBeginPlay
  (bind _returnvalue (Rendering|Material|CreateDynamicMaterialInstance (Variables|Default|GetCube) 0 0 "None" :!class /Script/Engine.PrimitiveComponent))
  (Variables|Default|SetMaterial _returnvalue)
  (Variables|Default|SetOriginalScale (Transformation|GetWorldScale (Variables|Default|GetCube))))

(fn ConstructionScript)