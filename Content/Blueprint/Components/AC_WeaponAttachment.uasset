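; Actor component that spawns weapons for its owner and attaches them to a given socket component.
; SpawnWeapon looks up the WeaponDataTable row named after the weapon class, spawns the actor, and passes in its projectile and fire-rate stats.
; It then attaches the weapon, initializes its projectiles and stores it in an array, from which GetWeaponActor returns the entry at the current index.
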(event Custom|SpawnWeapon
  (params (Socket :type Arrow%20Component%20Object%20Reference))
  (bind _spawnableweapon (Variables|Default|GetSpawnableWeapon))
  (bind _returnvalue (Utilities|GetDataTableRow (Variables|Default|GetWeapon_DataTable) (Utilities|String|StringToName (Utilities|String|Replace (Utilities|GetClassDisplayName _spawnableweapon) "_C")))
    (:then
      (bind _returnvalue_2 (Game|SpawnActorfromClass _spawnableweapon (Math|Transform|MakeTransform "0, 0, 0" "0, 0, 0" "1.000000,1.000000,1.000000") "Undefined" "MultiplyWithRoot" (Components|GetOwner) 0))
      (Default|InitializeData _returnvalue_2 (.ProjectileSpeed (Utilities|Struct|BreakF_WeaponData _returnvalue)) (.ProjectileLifespan (Utilities|Struct|BreakF_WeaponData _returnvalue)) (.ProjectileDamage (Utilities|Struct|BreakF_WeaponData _returnvalue)) (.ProjectileSpread (Utilities|Struct|BreakF_WeaponData _returnvalue)) (.ProjectileCount (Utilities|Struct|BreakF_WeaponData _returnvalue)) (.ProjectileHitCount (Utilities|Struct|BreakF_WeaponData _returnvalue)) (.ProjectileRadius (Utilities|Struct|BreakF_WeaponData _returnvalue)) (.MultishotAngleOffset (Utilities|Struct|BreakF_WeaponData _returnvalue)) (.FireRate (Utilities|Struct|BreakF_WeaponData _returnvalue)))
      (Transformation|AttachComponentToComponent _returnvalue_2 Socket "None" "KeepRelative" "KeepRelative" "KeepRelative" true)
      (Default|InitializeProjectiles _returnvalue_2)
      (Utilities|Array|Add (Variables|Default|GetWeaponActors) _returnvalue_2))
    (:RowNotFound
      (Development|PrintString "Hello"))))

(fn GetWeaponActor
  (return (Utilities|Array|Get(acopy) (Variables|Default|GetWeaponActors) (Variables|Default|GetCurrentWeaponIndex))))