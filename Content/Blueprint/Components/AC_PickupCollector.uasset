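; AC_PickupCollector is an actor component that tracks upgrade tiers for collected pickup types.
; OnPickupCollected converts the pickup enum to an index into parallel arrays of current tier, max tier, value and multiplier.
; IncrementTier raises the tier within its limit and reports whether it now exceeds the maximum.
; If not, the value grows by that type's multiplier; either way, OnStatsUpdated broadcasts type, tier and value, flagging maxed tiers.
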(event Custom|OnPickupCollected
  (params (Pickup :type E_Pickups%20Enum :default "NewEnumerator0"))
  (bind _output_get (Variables|Default|SetPickup Pickup))
  (bind _output_get_2 (Variables|Default|SetCurrentIndex (Math|Conversions|ToInteger(Byte) _output_get)))
  (bind _istiermaxed_ (Utilities|IncrementTier _output_get_2)
    (:Out
      (if (not _istiermaxed_)
        (Utilities|Array|SetArrayElem (Variables|Default|GetTierValue) (Variables|Default|GetCurrentIndex) (+ (Utilities|Array|Get(acopy) (Variables|Default|GetTierValue) (Variables|Default|GetCurrentIndex)) (* 1.0 (Utilities|Array|Get(acopy) (Variables|Default|GetTierValueMultiplier) (Variables|Default|GetCurrentIndex)))))
        (Default|CallOnStatsUpdated (Variables|Default|GetPickup) (Utilities|Array|Get(acopy) (Variables|Default|GetCurrentTier) (Variables|Default|GetCurrentIndex)) (Utilities|Array|Get(acopy) (Variables|Default|GetTierValue) (Variables|Default|GetCurrentIndex)) false)
        (else
          (Default|CallOnStatsUpdated (Variables|Default|GetPickup) (Utilities|Array|Get(acopy) (Variables|Default|GetCurrentTier) (Variables|Default|GetCurrentIndex)) (Utilities|Array|Get(acopy) (Variables|Default|GetTierValue) (Variables|Default|GetCurrentIndex)) true))))))